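; BP_SkvtScreen is a screen actor that displays a WBP_SkvtWeb widget through its Webpage component and can be turned off or destroyed.
; On BeginPlay it caches the widget reference.
; TurnOff forwards to that widget, retrying initialization first if the reference is invalid.
; EMPPulse destroys the Webpage component, leaving the actor in place, and spawns a smoke emitter at the actor's transform.
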(event `self.ReceiveBeginPlay`
  (`self.Initialize`))

(event `/Game/Skvt/Blueprints/BPI_ElectricDevice.TurnOff`
  (bind _webpageref (`self.WebpageRef`))
  (`/Engine/EditorBlueprintResources/StandardMacros.IsValid` _webpageref :!label _label
    (:`Is Valid`
      (`/Game/Skvt/Blueprints/Screen/WBP_SkvtWeb.TurnOff` _webpageref))
    (:`Is Not Valid`
      (`self.Initialize`)
      (goto _label))))

(event `/Game/Skvt/Blueprints/BPI_ElectricDevice.EMPPulse`
  (`self.DestroyScreen`))

(fn `DestroyScreen`
  (`ActorComponent.K2_DestroyComponent` (`self.Webpage`))
  (`self.SpawnDestroyedEffect`))

(fn `Initialize`
  (bind _aswbp_skvt_web (cast `/Game/Skvt/Blueprints/Screen/WBP_SkvtWeb` (`WidgetComponent.GetWidget` (`self.Webpage`))))
  (set `self.WebpageRef` _aswbp_skvt_web))

(fn `SpawnDestroyedEffect`
  (bind (_returnvalue_location _returnvalue_rotation) (`KismetMathLibrary.BreakTransform` (`self.GetTransform`)))
  (`GameplayStatics.SpawnEmitterAtLocation` "/Game/StarterContent/Particles/P_Smoke.P_Smoke" _returnvalue_location _returnvalue_rotation))

(fn `UserConstructionScript`)