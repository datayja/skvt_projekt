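; BP_SkvtGameMode is a game mode that hands player control to another living character, or brings up the main menu when none remain.
; It caches the Skvt player controller on BeginPlay.
; PossessNextCharacter uses FindValidCharacter, which returns the first BP_SkvtBaseChar in the world that is not dead, then has the controller possess it or create the main menu.
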(event `self.ReceiveBeginPlay`
  (bind _asbp_skvt_player_controller (cast `/Game/Skvt/Characters/BP_SkvtPlayerController` (`GameplayStatics.GetPlayerController` 0)))
  (set `self.PlayerController` _asbp_skvt_player_controller))

(event `PossessNextCharacter`
  (bind _newpawn (`self.FindValidCharacter`))
  (`/Engine/EditorBlueprintResources/StandardMacros.IsValid` _newpawn
    (:`Is Valid`
      (`Controller.Possess` (`self.PlayerController`) _newpawn))
    (:`Is Not Valid`
      (`/Game/Skvt/Characters/BP_SkvtPlayerController.CreateMainMenu` (`self.PlayerController`)))))

(fn `FindValidCharacter`
  (returns (NewPawn :type "Pawn Object Reference"))
  (bind _outactors (`GameplayStatics.GetAllActorsOfClass` "/Game/Skvt/Characters/BP_SkvtBaseChar.BP_SkvtBaseChar_C"))
  (if (`KismetArrayLibrary.Array_IsNotEmpty` _outactors)
    (for _array_element _outactors
      (if (not (`/Game/Skvt/Characters/BP_SkvtBaseChar.IsDead` _array_element))
        (return _array_element)))))

(fn `UserConstructionScript`)