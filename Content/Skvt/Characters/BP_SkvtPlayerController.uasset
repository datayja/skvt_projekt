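; Player controller for Skvt that registers input mappings, cycles possession between pawns and toggles the main menu.
; On BeginPlay it adds the PMI_SkvtMapping config to the Enhanced Input subsystem.
; The swap action possesses the next pawn from GetAllActorsOfClass, wrapping to the first.
; The menu action creates WBP_MainMenu with pause, cursor and Game-and-UI input, or delegates closing to the widget's CloseMenu.
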(event `self.ReceiveBeginPlay`
  (`self.AddMappingContexts`))

(event `EnhancedInput|/Game/Skvt/Characters/Input/Actions/IA_Swap`
  (params (ActionValue :type Boolean) (ElapsedSeconds :type "Float (double-precision)") (TriggeredSeconds :type "Float (double-precision)") (InputAction :type "InputAction Object Reference" :default "/Game/Skvt/Characters/Input/Actions/IA_Swap.IA_Swap"))
  (:`Triggered`
    (bind _outactors (`GameplayStatics.GetAllActorsOfClass` "/Script/Engine.Pawn"))
    (`self.Possess` (`self.GetPawnToPossess` _outactors))))

(event `EnhancedInput|/Game/Skvt/Characters/Input/Actions/IA_OpenMenu`
  (params (ActionValue :type Boolean) (ElapsedSeconds :type "Float (double-precision)") (TriggeredSeconds :type "Float (double-precision)") (InputAction :type "InputAction Object Reference" :default "/Game/Skvt/Characters/Input/Actions/IA_OpenMenu.IA_OpenMenu"))
  (:`Triggered`
    (if (`self.IsMainMenuOpen`)
      (`self.CloseMainMenu`)
      (else
        (`self.CreateMainMenu`)))))

(fn `AddMappingContexts`
  (bind _returnvalue (pcsubsystem `EnhancedInputLocalPlayerSubsystem` self))
  (`/Engine/EditorBlueprintResources/StandardMacros.IsValid` _returnvalue
    (:`Is Valid`
      (`EnhancedInputSubsystemInterface.AddPlayerMappableConfig` _returnvalue "/Game/Skvt/Characters/Input/PMI_SkvtMapping.PMI_SkvtMapping" (struct)))))

(fn `CloseMainMenu`
  (`/Game/Skvt/UI/Widgets/Menu/WBP_MainMenu.CloseMenu` (`self.MenuWidget`))
  (set `self.MenuWidget` null))

(fn `CreateMainMenu`
  (bind _returnvalue (`|CreateWidget` "/Game/Skvt/UI/Widgets/Menu/WBP_MainMenu.WBP_MainMenu_C" self))
  (bind _output_get (set `self.MenuWidget` _returnvalue))
  (`UserWidget.AddToViewport` _output_get 0)
  (`WidgetBlueprintLibrary.SetInputMode_GameAndUIEx` self _output_get)
  (`GameplayStatics.SetGamePaused` true)
  (set `self.bShowMouseCursor` true))

(fn `GetPawnToPossess`
  (params (PawnAray :type "Array of Pawn Object Reference"))
  (returns (Pawn :type "Pawn Object Reference"))
  (bind _returnvalue (+ (`KismetArrayLibrary.Array_Find` PawnAray (`self.K2_GetPawn`)) 1))
  (if (`KismetArrayLibrary.Array_IsValidIndex` PawnAray _returnvalue)
    (return (`|GetArrayItem` (`local.PawnAray`) _returnvalue))
    (else
      (return (`|GetArrayItem` (`local.PawnAray`))))))

(fn `IsMainMenuOpen`
  (returns (IsOpen :type Boolean))
  (return (`KismetSystemLibrary.IsValid` (`self.MenuWidget`))))

(fn `UserConstructionScript`)